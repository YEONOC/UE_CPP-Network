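; BP_ColorBox is a replicated box actor that changes to a random color when something begins overlapping its Box component.
; BeginPlay gives the mesh a dynamic instance of M_Color.
; The overlap calls ChangeToRandomColor, which only on authority picks a random BoxColor and sets the material's Color parameter.
; OnRep_BoxColor applies the replicated color to the material on clients.
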(event OnComponentBeginOverlap(Box)
  (params (OverlappedComponent :type Primitive%20Component%20Object%20Reference) (OtherActor :type Actor%20Object%20Reference) (OtherComp :type Primitive%20Component%20Object%20Reference) (OtherBodyIndex :type Integer) (bFromSweep :type Boolean) (SweepResult :type Hit%20Result%20Structure%20%28by%20ref%29))
  (CallFunction|ChangetoRandomColor))

(event Custom|ChangeToRandomColor
  (Networking|SwitchHasAuthority
    (:Authority
      (bind _output_get (Variables|Default|SetBoxColor (Math|Color|MakeColor (Math|Random|RandomFloatinRange 0.0 1.0) (Math|Random|RandomFloatinRange 0.0 1.0) (Math|Random|RandomFloatinRange 0.0 1.0))))
      (Rendering|Material|SetVectorParameterValue (Variables|Default|GetMI_Color) "Color" _output_get :!class /Script/Engine.MaterialInstanceDynamic))))

(event EventBeginPlay
  (bind _returnvalue (Rendering|Material|CreateDynamicMaterialInstance (Variables|Character|GetMesh) 0 "/Game/Materials/M_Color.M_Color" "None" :!class /Script/Engine.PrimitiveComponent))
  (bind _output_get (Variables|Default|SetMI_Color _returnvalue))
  (Rendering|Material|SetMaterial (Variables|Character|GetMesh) 0 _output_get))

(fn ConstructionScript)

(fn OnRepBoxColor
  (Rendering|Material|SetVectorParameterValue (Variables|Default|GetMI_Color) "Color" (Variables|Default|GetBoxColor) :!class /Script/Engine.MaterialInstanceDynamic))